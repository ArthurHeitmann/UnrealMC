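; BP_ItemDrop is a debugging-tool actor for a dropped item that falls under physics.
; The construction script builds a procedural Mesh section from its Verts, Tris and UVs variables, leaving Normals unused.
; BeginPlay enables gravity and physics simulation on both Mesh and the SM component, overrides Mesh mass, and wakes their rigid bodies.
; A node to move Mesh to SM's location is disconnected, so nothing in the graph keeps them aligned.
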(event EventBeginPlay
  (Physics|SetEnableGravity (Variables|Character|GetMesh) true)
  (Physics|SetEnableGravity (Variables|Default|GetSM) true)
  (Class|PrimitiveComponent|SetMassOverrideinKg (Variables|Character|GetMesh) "None" 5e+01 true)
  (Physics|SetSimulatePhysics (Variables|Default|GetSM) true)
  (Physics|SetSimulatePhysics (Variables|Character|GetMesh) true)
  (Class|PrimitiveComponent|WakeAllRigidBodies (Variables|Default|GetSM))
  (Class|PrimitiveComponent|WakeAllRigidBodies (Variables|Character|GetMesh)))

(event Collision|EventActorBeginOverlap
  (params (OtherActor :type Actor%20Object%20Reference)))

(event EventTick
  (params (DeltaSeconds :type Float%20%28single-precision%29)))

(fn ConstructionScript
  (Class|ProceduralMeshComponent|CreateMeshSectionLinearColor (Variables|Character|GetMesh) 0 (Variables|Default|GetVerts) (Variables|Default|GetTris) 0 (Variables|Default|GetUVs) 0 0 0 0 0 false))